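; Gameplay player controller for Into the Limbo that spawns the player's selected character and relays pause requests.
; On BeginPlay it loads player info and the character choice from the Steam game instance, then spawns and possesses that character at a PlayerStart.
; Pause and unpause go to the game mode for everyone, while a separate event forwards pause state to the ThirdPerson or Shadow character.
; It also handles exiting to the main menu.
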(event Custom|Load%20Player%20Info
  ;[1 1 1] Load Player Info
  (bind _game_instance (Class|BPIMainMenu|SteamGameInstanceRef(Message) (Game|GetGameInstance)))
  (bind _playerinfo (Class|BPIMainMenu|LoadPlayerInfo(Message) _game_instance))
  (bind _output_get (Variables|Default|SetPlayerInfo _playerinfo))
  (Utilities|Struct|SetmembersinS_PlayerInfo _output_get)
  (CallFunction|PossessPlayerCharacterClient (Variables|/Game/ThirdPersonBP/Blueprints/IntoTheLimbo_GameInstance.IntoTheLimbo_GameInstance_C|GetSelectedCharacter _game_instance) self))

(event Custom|Possess%20Player%20Character%20Client
  (params (Selected%20Character :type Character%20Class%20Reference) (Player%20Controller :type Player%20Controller%20Object%20Reference))
  ;[1 1 1] Player Controller Posseses Character Selected
  (CallFunction|PossessPlayerCharacterServer Selected%20Character Player%20Controller))

(event Custom|Possess%20Player%20Character%20Server
  (params (Character%20Selected :type Character%20Class%20Reference) (Player%20Controller :type Player%20Controller%20Object%20Reference))
  ;[1 1 1] Player Controller Posseses Character Selected
  (bind _returnvalue (Actor|GetActorOfClass "/Script/Engine.PlayerStart"))
  (bind _returnvalue_2 (Game|SpawnActorfromClass Character%20Selected (Transformation|GetActorTransform _returnvalue) "Undefined" 0 0))
  (Pawn|Possess Player%20Controller _returnvalue_2))

(event Custom|PauseGameInCharacter
  (params (Pause :type Boolean) (PlayerPausedName :type String))
  (bind _returnvalue (Game|GetPlayerCharacter 0))
  ;[1 1 1] Pause Game
  (bind _asthird_person_character (Utilities|Casting|CastToThirdPersonCharacter _returnvalue)
    (:then
      (Default|PauseGame _asthird_person_character Pause PlayerPausedName))
    (:CastFailed
      (bind _asshadow_person_character (Utilities|Casting|CastToShadowPersonCharacter _returnvalue)
        (:then
          (Default|PauseGame _asshadow_person_character Pause PlayerPausedName))
        (:CastFailed
          (Development|PrintString "Cast Failed Totaly"))))))

(event Custom|UnpausedGame
  ;[1 1 1] Pause and Unpausa Game
  (CallFunction|UnpausedGameGM self))

(event Custom|UnpausedGameGM
  (params (PlayerPaused :type BP%20Gameplay%20Player%20Controller%20Object%20Reference))
  ;[1 1 1] Pause and Unpausa Game
  (bind _intothelimbogm (Class|BPIGameplayGameMode|IntotheLimboGMRef(Message) (Game|GetGameMode)))
  (Default|UnpausedGameforEveryone _intothelimbogm PlayerPaused))

(event Custom|PauseGame
  ;[1 1 1] Pause and Unpausa Game
  (Development|PrintString "PauseGame PC" true true "(R=0.000000,G=0.660000,B=1.000000,A=1.000000)" 5.0)
  (CallFunction|PauseGameGM self (Utilities|String|ToString(Text) (Utilities|Struct|BreakS_PlayerInfo (Variables|Default|GetPlayerInfo)))))

(event Custom|PauseGameGM
  (params (PlayerPaused :type BP%20Gameplay%20Player%20Controller%20Object%20Reference) (PlayerPausedGame :type String))
  ;[1 1 1] Pause and Unpausa Game
  (Development|PrintString "Hello PauseGameGM")
  (bind _intothelimbogm (Class|BPIGameplayGameMode|IntotheLimboGMRef(Message) (Game|GetGameMode)))
  (Default|PauseGameforEveryone _intothelimbogm PlayerPaused PlayerPausedGame))

(event Custom|ExitToMainMenu
  ;[1 1 1] Exit to Main Menu
  (Game|OpenLevel(byName) "Main_Menu_Lvl"))

(event EventBeginPlay
  ;[1 1 1] Event Begin Play
  (Development|PrintString "Gameplayer Controller Begin Play")
  (CallFunction|LoadPlayerInfo)
  (Viewport|RemoveAllWidgets)
  (Input|SetInputModeGameOnly self))

(fn ConstructionScript)

(fn GameplayPCRef
  (return self))